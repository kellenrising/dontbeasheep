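; Player-controllable sheep pawn Blueprint that handles basic directional movement.
; The forward and right input axes call AddMovementInput along vectors built from the control rotation's yaw only, so camera pitch and roll do not affect direction.
; Both axes are ignored while the MovementDisabled flag is set.
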(event `InputAxis|forward`
  (params (AxisValue :type "Float (single-precision)"))
  ;[1 1 1] Movement
  (if (not (`self.MovementDisabled`))
    (`self.AddMovementInput` (`KismetMathLibrary.GetForwardVector` (`KismetMathLibrary.MakeRotator` 0.0 0.0 (.yaw (`self.GetControlRotation`)))) AxisValue)))

(event `InputAxis|right`
  (params (AxisValue :type "Float (single-precision)"))
  ;[1 1 1] Movement
  (if (not (`self.MovementDisabled`))
    (`self.AddMovementInput` (`KismetMathLibrary.GetRightVector` (`KismetMathLibrary.MakeRotator` 0.0 0.0 (.yaw (`self.GetControlRotation`)))) AxisValue)))

(fn `UserConstructionScript`)