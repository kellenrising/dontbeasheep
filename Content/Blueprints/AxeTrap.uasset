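; Axe trap Blueprint that swings two axes when a Bp_sheep011 actor overlaps its DetectPlayer component.
; The RotateAxes timeline pitches the axes in opposite directions, then after a three-second delay Timeline_0 drives them with its own track.
; TrapTripped works as an armed flag, cleared on trigger and set again on every Timeline_0 update.
; Timeline_0 uses Play rather than PlayFromStart, and the graph contains no damage logic.
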(event `self.DetectPlayer.OnComponentBeginOverlap`
  (params (OverlappedComponent :type "PrimitiveComponent Object Reference") (OtherActor :type "Actor Object Reference") (OtherComp :type "PrimitiveComponent Object Reference") (OtherBodyIndex :type Integer) (bFromSweep :type Boolean) (SweepResult :type "HitResult Structure (by ref)"))
  (if (== (`GameplayStatics.GetObjectClass` OtherActor) "/Game/Blueprints/bp_sheep011.bp_sheep011_C")
    (if (`self.trapTripped`)
      (set `self.trapTripped` false)
      (bind (_direction _newtrack_0) (`Timeline|rotate axes` :!via `PlayFromStart`)
        (:`Update`
          (`SceneComponent.K2_SetWorldRotation` (`self.Axe1`) (`KismetMathLibrary.MakeRotator` 0.0 _newtrack_0 90.0) false false)
          (`SceneComponent.K2_SetWorldRotation` (`self.Axe2`) (`KismetMathLibrary.MakeRotator` 0.0 (* _newtrack_0 -1.0) 90.0) false false))
        (:`Finished`
          (`KismetSystemLibrary.Delay` 3.0)
          (bind (_direction_2 _newtrack_0_2) (`Timeline|Timeline_0`)
            (:`Update`
              (`SceneComponent.K2_SetWorldRotation` (`self.Axe1`) (`KismetMathLibrary.MakeRotator` 0.0 _newtrack_0_2 90.0) false false)
              (`SceneComponent.K2_SetWorldRotation` (`self.Axe2`) (`KismetMathLibrary.MakeRotator` 0.0 (* _newtrack_0_2 -1.0) 90.0) false false)
              (set `self.trapTripped` true))))))))

(fn `UserConstructionScript`)