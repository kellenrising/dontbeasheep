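; Behavior Tree task that moves the sheep AI's pawn to the character stored in the TargetObject blackboard key.
; It caches the SheepAIController from the owner, then runs AIMoveTo toward the target's capsule component location to avoid a pathing bug.
; The task finishes only when the move succeeds, with no handling for failed moves or casts.
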(event `self.ReceiveExecute`
  (params (OwnerActor :type "Actor Object Reference"))
  ;[1 1 1] Check if ref not null
  (if (not (!= null null))
    (bind _assheep_aicontroller (cast `/Game/Blueprints/AI/SheepAIController` OwnerActor))
    (set `self.SheepAIController_Ref` _assheep_aicontroller))
  ;[1 1 1] getting the capsule collision's location to avoid pathing bug
  (bind _ascharacter (cast `Character` (`BTFunctionLibrary.GetBlackboardValueAsActor` (`self.TargetObject`))))
  (`|AIMoveTo` (`Controller.K2_GetPawn` (`self.SheepAIController_Ref`)) (`SceneComponent.K2_GetComponentLocation` (`Character.CapsuleComponent` _ascharacter)) null (`self.MoveToAcceptanceRadius`)
    (:`OnSuccess`
      (`self.FinishExecute` true))))