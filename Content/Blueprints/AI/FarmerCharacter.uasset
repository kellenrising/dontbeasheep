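; Enemy farmer character that attacks the player with bullets and a one-time pitchfork throw.
; Tick tracks player distance and fires Attack on a timer when in range, setting IsAttacking around a movement pause.
; Close range randomly picks single, spread or unrolled Delay-chain gatling shots; farther away prefers the pitchfork, then spread or gatling.
; Bp_sqwer overlaps add damage with sound and blood; the third enlarges the blood burst and rotates the farmer.
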(event `self.ReceiveTick`
  (params (DeltaSeconds :type "Float (single-precision)"))
  ;[1 0.8422 0.1435] On tick
  (set `self.DistanceFromPlayer` (`KismetMathLibrary.VSize` (- (`self.K2_GetActorLocation`) (`self.K2_GetActorLocation` (`GameplayStatics.GetPlayerPawn` 0)))))
  (set `self.isPlayerInRange` (<= (`self.DistanceFromPlayer`) (`self.PlayerFollowRange`)))
  (bind _output_get (set `self.ElapsedTime` (+ DeltaSeconds (`self.ElapsedTime`))))
  (if (>= _output_get (`self.NormalFireRate`))
    (set `self.ElapsedTime` (- (`self.ElapsedTime`) (`self.NormalFireRate`)))
    (if (`self.isPlayerInRange`)
      (`self.Attack`))))

(event `ShootNormal`
  ;[1 1 1] Shooting normally once
  (`self.Shoot` (`self.ProjectileSpawnPoint`)))

(event `Shoot`
  (params (ArrowReference :type "ArrowComponent Object Reference"))
  ;[1 1 1] Shooting
  (`|SpawnActorFromClass` (`self.BulletProjectile`) (`SceneComponent.K2_GetComponentToWorld` ArrowReference) "Undefined" "OverrideRootScale" null (`self.BulletSpeed`) (`self.BulletGravityScale`)))

(event `ThrowPitchfork`
  ;[1 1 1] Throwing the pitchfork
  (if (`self.hasPitchfork`)
    (`|SpawnActorFromClass` (`self.PitchforkProjectile`) (`SceneComponent.K2_GetComponentToWorld` (`self.ProjectileSpawnPoint`)) "Undefined" "OverrideRootScale" null (`self.PitchforkSpeed`) (`self.PitchforkGravityScale`))
    (set `self.hasPitchfork` false)))

(event `SpreadShot`
  ;[1 1 1] Multi-bullet spread shot
  (`|ExecutionSequence`
    (:`then_0`
      (`self.Shoot` (`self.ProjectileSpawnPoint`)))
    (:`then_1`
      (`self.Shoot` (`self.Spread1`)))
    (:`then_2`
      (`self.Shoot` (`self.Spread2`)))
    (:`then_3`
      (`self.Shoot` (`self.Spread3`)))
    (:`then_4`
      (`self.Shoot` (`self.Spread4`)))))

(event `Attack`
  ;[1 1 1] Choosing an action
  (set `self.isAttacking` true)
  (if (<= (`self.DistanceFromPlayer`) (`self.BufferDistanceFromPlayer`))
    (switch `int` (`KismetMathLibrary.RandomIntegerInRange` 0 2)
      (:`0`
        (`self.ShootNormal`))
      (:`1`
        (`self.SpreadShot`))
      (:`2`
        (`self.ShootGatling`)))
    (elif (`self.hasPitchfork`)
      (`self.ThrowPitchfork`)
      (else
        (switch `int` (`KismetMathLibrary.RandomIntegerInRange` 0 1)
          (:`0`
            (`self.SpreadShot`))
          (:`1`
            (`self.ShootGatling`))))))
  (`KismetSystemLibrary.Delay` (`self.AttackingMovementPauseTime`))
  (set `self.isAttacking` false))

(event `ShootGatling`
  (bind _gatlingdelay (`self.GatlingDelay`))
  ;[1 1 1] gatling
  ; TO DO: make for loop macro with delay functionality
  (`self.ShootNormal`)
  (`KismetSystemLibrary.Delay` _gatlingdelay)
  (`self.ShootNormal`)
  (`KismetSystemLibrary.Delay` _gatlingdelay)
  (`self.ShootNormal`)
  (`KismetSystemLibrary.Delay` _gatlingdelay)
  (`self.ShootNormal`)
  (`KismetSystemLibrary.Delay` _gatlingdelay)
  (`self.ShootNormal`)
  (`KismetSystemLibrary.Delay` _gatlingdelay)
  (`self.ShootNormal`)
  (`KismetSystemLibrary.Delay` _gatlingdelay)
  (`self.ShootNormal`)
  (`KismetSystemLibrary.Delay` _gatlingdelay)
  (`self.ShootNormal`)
  (`KismetSystemLibrary.Delay` _gatlingdelay)
  (`self.ShootNormal`)
  (`KismetSystemLibrary.Delay` _gatlingdelay)
  (`self.ShootNormal`)
  (`KismetSystemLibrary.Delay` _gatlingdelay)
  (`self.ShootNormal`)
  (`KismetSystemLibrary.Delay` _gatlingdelay)
  (`self.ShootNormal`)
  (`KismetSystemLibrary.Delay` _gatlingdelay)
  (`self.ShootNormal`)
  (`KismetSystemLibrary.Delay` _gatlingdelay))

(event `self.Mesh.OnComponentBeginOverlap`
  (params (OverlappedComponent :type "PrimitiveComponent Object Reference") (OtherActor :type "Actor Object Reference") (OtherComp :type "PrimitiveComponent Object Reference") (OtherBodyIndex :type Integer) (bFromSweep :type Boolean) (SweepResult :type "HitResult Structure (by ref)"))
  (bind _returnvalue (`self.K2_GetActorLocation`))
  (if (== (`GameplayStatics.GetObjectClass` OtherActor) "/Game/Blueprints/bp_sqwer.bp_sqwer_C")
    (`GameplayStatics.PlaySoundAtLocation` "/Game/Sounds/death_sound.death_sound" _returnvalue)
    (`GameplayStatics.SpawnEmitterAtLocation` "/Game/Particles/blood_particles.blood_particles" _returnvalue)
    (bind _output_get (set `self.Damage` (+ (`self.Damage`) 1)))
    (`/Engine/EditorBlueprintResources/StandardMacros.CompareInt` _output_get 3
      (:`==`
        (bind _returnvalue_2 (`GameplayStatics.SpawnEmitterAtLocation` "/Game/Particles/blood_particles.blood_particles" _returnvalue))
        (`SceneComponent.SetRelativeScale3D` _returnvalue_2 (10.0 10.0 10.0))
        (`self.K2_SetActorRotation` (struct :`Pitch` 90.0))))))

(fn `UserConstructionScript`)