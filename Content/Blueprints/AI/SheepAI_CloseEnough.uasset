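; Behavior tree decorator for the sheep AI that gates a branch on the pawn's distance to a target actor.
; It casts the owner to SheepAIController, caches it, and measures from the controlled pawn to the actor in the TargetObject blackboard key.
; Despite the CloseEnough name, the condition passes when that distance is at least AcceptableDistance, meaning the sheep is not yet inside the range.
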(fn `PerformConditionCheck`
  (params (OwnerActor :type "Actor Object Reference"))
  (returns (ReturnValue :type Boolean))
  (bind _assheep_aicontroller (cast `/Game/Blueprints/AI/SheepAIController` OwnerActor))
  (set `self.SheepAIController_Ref` _assheep_aicontroller)
  (return (>= (`KismetMathLibrary.VSize` (- (`Actor.K2_GetActorLocation` (`BTFunctionLibrary.GetBlackboardValueAsActor` (`self.TargetObject`))) (`Actor.K2_GetActorLocation` (`Controller.K2_GetPawn` (`self.SheepAIController_Ref`))))) (`self.AcceptableDistance`))))