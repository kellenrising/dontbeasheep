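; Sheep AI behavior tree node that looks for visible target objects around the controlled pawn on each tick.
; It caches the SheepAIController, then runs a vertical multi-sphere trace for configured object types, ignoring all sheep characters.
; A visibility line trace checks each hit, setting TargetObject and TargetLocation when unobstructed and clearing only TargetObject otherwise.
; The loop never breaks, so the last hit decides TargetObject.
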(event `self.ReceiveTick`
  (params (OwnerActor :type "Actor Object Reference") (DeltaSeconds :type "Float (single-precision)"))
  (bind _returnvalue (`Actor.K2_GetActorLocation` (`Controller.K2_GetPawn` (`self.SheepAIController_Ref`))))
  ;[1 1 1] Check that reference is not null
  (if (not (!= (`self.SheepAIController_Ref`) null))
    (bind _assheep_aicontroller (cast `/Game/Blueprints/AI/SheepAIController` OwnerActor))
    (set `self.SheepAIController_Ref` _assheep_aicontroller))
  (bind _outactors (`GameplayStatics.GetAllActorsOfClass` "/Game/Blueprints/AI/SheepAICharacter.SheepAICharacter_C"))
  (set `self.MyLocation` _returnvalue)
  (bind _outhits (`KismetSystemLibrary.SphereTraceMultiForObjects` _returnvalue (+ _returnvalue (`KismetMathLibrary.MakeVector` 0.0 0.0 (`self.SphereTraceZHeight`))) (`self.SphereTraceRadius`) (`self.DesiredObjectTypes`) false _outactors))
  (for _array_element _outhits
    (bind (_bblockinghit _binitialoverlap _time _location _impactpoint _normal _impactnormal _physmat _hitactor) (`GameplayStatics.BreakHitResult` _array_element))
    (bind _outhit (`KismetSystemLibrary.LineTraceSingle` (`self.MyLocation`) (`Actor.K2_GetActorLocation` _hitactor) "TraceTypeQuery1" false _outactors))
    (bind (_bblockinghit_2 _binitialoverlap_2 _time_2 _location_2 _impactpoint_2 _normal_2 _impactnormal_2 _physmat_2 _hitactor_2) (`GameplayStatics.BreakHitResult` _outhit))
    (if (== _hitactor_2 _hitactor)
      (`BTFunctionLibrary.SetBlackboardValueAsObject` (`self.TargetObject`) _hitactor_2)
      (`BTFunctionLibrary.SetBlackboardValueAsVector` (`self.TargetLocation`) (`Actor.K2_GetActorLocation` _hitactor_2))
      (else
        (`BTFunctionLibrary.SetBlackboardValueAsObject` (`self.TargetObject`))))))