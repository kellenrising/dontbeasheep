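; AI controller for the farmer character that chases and faces the player.
; Each tick it reads the pawn's range, attack and distance state, and acts only while the player is in range.
; It moves toward the player's location when not attacking and beyond the buffer distance.
; Otherwise it stops and snaps its rotation to look straight at the player.
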(event `self.ReceiveTick`
  (params (DeltaSeconds :type "Float (single-precision)"))
  ;[1 0.9342 0.1995] on tick
  (bind _asfarmer_character (cast `/Game/Blueprints/AI/FarmerCharacter` (`self.K2_GetPawn`)))
  (if (`/Game/Blueprints/AI/FarmerCharacter.isPlayerInRange` _asfarmer_character)
    (if (and (not (`/Game/Blueprints/AI/FarmerCharacter.isAttacking` _asfarmer_character)) (> (`/Game/Blueprints/AI/FarmerCharacter.DistanceFromPlayer` _asfarmer_character) (`/Game/Blueprints/AI/FarmerCharacter.BufferDistanceFromPlayer` _asfarmer_character)))
      (`self.MoveToPlayer`)
      (else
        (`self.StopMovement`)
        (`self.RotateToFacePlayer`)))))

(event `MoveToPlayer`
  ;[1 1 1] move to player
  (`self.MoveToLocation` (`self.K2_GetActorLocation` (`GameplayStatics.GetPlayerPawn` 0))))

(event `RotateToFacePlayer`
  (bind _returnvalue (`self.K2_GetPawn`))
  ;[1 1 1] rotate to face player
  (`self.K2_SetActorRotation` _returnvalue (`KismetMathLibrary.FindLookAtRotation` (`self.K2_GetActorLocation` _returnvalue) (`self.K2_GetActorLocation` (`GameplayStatics.GetPlayerPawn` 0))) false))

(fn `UserConstructionScript`)