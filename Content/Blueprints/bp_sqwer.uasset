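; A saw trap combined with a trigger button that opens a linked gate for the sheep.
; Tick constantly spins the saw meshes, while a self-recalling cycle pops the Sphere component up and down with sound and randomized delays.
; Any Trigger overlap starts that cycle; a Bp_sheep011 overlap also disables the trigger, opens the bp_gate and turns the red button green.
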(event `self.ReceiveTick`
  (params (DeltaSeconds :type "Float (single-precision)"))
  ;[1 1 1] spin
  (`SceneComponent.K2_AddLocalRotation` (`self.Saw`) (struct :`Pitch` 20.0) false false)
  (`SceneComponent.K2_AddLocalRotation` (`self.StaticMesh`) (struct :`Pitch` 20.0) false false)
  (`SceneComponent.K2_AddLocalRotation` (`self.StaticMesh1`) (struct :`Pitch` 20.0) false false))

(event `self.ReceiveBeginPlay`)

(event `sawCycle`
  ;[1 1 1] Saw cycle
  (`KismetSystemLibrary.Delay` (`KismetMathLibrary.RandomFloatInRange` 0.2 0.7))
  (`GameplayStatics.PlaySoundAtLocation` null (`self.K2_GetActorLocation`))
  (`KismetSystemLibrary.MoveComponentTo` (`self.Sphere`) (0.0 0.0 50.0) (struct) false false 0.1 true)
  (`KismetSystemLibrary.Delay` (`KismetMathLibrary.RandomFloatInRange` 1.0 2.0))
  (`KismetSystemLibrary.MoveComponentTo` (`self.Sphere`) (0.0 0.0 -100.0) (struct) false false 0.1 true)
  (`KismetSystemLibrary.Delay` 2.0)
  (`self.sawCycle`))

(event `self.trigger.OnComponentBeginOverlap`
  (params (OverlappedComponent :type "PrimitiveComponent Object Reference") (OtherActor :type "Actor Object Reference") (OtherComp :type "PrimitiveComponent Object Reference") (OtherBodyIndex :type Integer) (bFromSweep :type Boolean) (SweepResult :type "HitResult Structure (by ref)"))
  ;[1 1 1] Comment
  (`self.sawCycle`)
  (if (== (`GameplayStatics.GetObjectClass` OtherActor) "/Game/Blueprints/bp_sheep011.bp_sheep011_C")
    (`PrimitiveComponent.SetCollisionEnabled` (`self.trigger`) "NoCollision")
    (bind _asbp_gate (cast `/Game/Blueprints/bp_gate` (`self.Gate`))
      (:`then`
        (set `self.key1Unlocked` true)
        (`/Game/Blueprints/bp_gate.Open` _asbp_gate)
        (`StaticMeshComponent.SetStaticMesh` (`self.Red_button`) "/Game/Models/Green_Button.Green_Button")
        (set `self.key1Unlocked` false))
      (:`CastFailed`
        (`KismetSystemLibrary.PrintString` "no dice")))))

(event `saw3`)

(event `saw2`)

(fn `UserConstructionScript`)