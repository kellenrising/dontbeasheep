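; TimedSaws is a moving, spinning saw actor that bounces back and forth within a stretch of the level.
; BeginPlay randomizes its Y velocity, then Tick adds yaw by a fixed per-frame step and sweeps it along its velocity.
; X velocity flips on every tick spent outside two hardcoded world-X bounds, while any overlap on its static mesh flips Y velocity.
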(event `self.ReceiveBeginPlay`
  (set `self.velocity` (`KismetMathLibrary.MakeVector` (.x (`self.velocity`)) (* (.y (`self.velocity`)) (`KismetMathLibrary.RandomFloatInRange` -2.0 2.0)) (.z (`self.velocity`)))))

(event `self.ReceiveTick`
  (params (DeltaSeconds :type "Float (single-precision)"))
  (bind _x (.x (`self.K2_GetActorLocation`)))
  (bind _output_get (set `self.rotate` (+ (`self.rotate`) 2.0)))
  (`self.K2_SetActorTransform` (`KismetMathLibrary.MakeTransform` (+ (`self.K2_GetActorLocation`) (* (`self.velocity`) DeltaSeconds)) (`KismetMathLibrary.MakeRotator` 0.0 0.0 _output_get)) true)
  (`/Engine/EditorBlueprintResources/StandardMacros.CompareFloat` _x -4222.767578
    (:`>`
      (`/Engine/EditorBlueprintResources/StandardMacros.CompareFloat` _x -2379.495117
        (:`>`
          _)
        (:`==`
          _)))
    (:`==`
      _)
    (:`<`
      _))
  (set `self.velocity` (`KismetMathLibrary.MakeVector` (* (.x (`self.velocity`)) -1.0) (.y (`self.velocity`)) (.z (`self.velocity`)))))

(event `self.StaticMesh.OnComponentBeginOverlap`
  (params (OverlappedComponent :type "PrimitiveComponent Object Reference") (OtherActor :type "Actor Object Reference") (OtherComp :type "PrimitiveComponent Object Reference") (OtherBodyIndex :type Integer) (bFromSweep :type Boolean) (SweepResult :type "HitResult Structure (by ref)"))
  (set `self.velocity` (`KismetMathLibrary.MakeVector` (.x (`self.velocity`)) (* (.y (`self.velocity`)) -1.0) (.z (`self.velocity`)))))

(fn `UserConstructionScript`)