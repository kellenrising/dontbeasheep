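; Gate actor that removes itself, as an opened fence, once its unlock count reaches seven.
; The Open event loops over the Sqwer01 array, casts each element to bp_sqwer and counts those flagged Key1Unlocked, with every key case incrementing alike.
; The count is checked after each increment and resets only on reaching seven, so it carries across calls.
; Debug strings report the count, success and failed casts.
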(event `Open`
  (bind _unlocked (`self.Unlocked`))
  (bind _unlocked_2 (`self.unlocked`))
  ;[1 1 1] OPEN THAT DOOR
  (for _array_element (`self.sqwer01`)
    (bind _asbp_sqwer (cast `/Game/Blueprints/bp_sqwer` _array_element)
      (:`then`
        (if (`/Game/Blueprints/bp_sqwer.key1Unlocked` _asbp_sqwer)
          (switch `/Game/enumeration/Keys` (`/Game/Blueprints/bp_sqwer.Keys Unlocked` _asbp_sqwer)
            (:`NewEnumerator0`
              (set `self.Unlocked` (+ _unlocked_2 1)))
            (:`NewEnumerator1`
              (set `self.Unlocked` (+ _unlocked_2 1)))
            (:`NewEnumerator2`
              (set `self.Unlocked` (+ _unlocked_2 1)))
            (:`NewEnumerator3`
              (set `self.Unlocked` (+ _unlocked_2 1)))
            (:`NewEnumerator4`
              (set `self.Unlocked` (+ _unlocked_2 1)))
            (:`NewEnumerator5`
              (set `self.Unlocked` (+ _unlocked_2 1)))
            (:`NewEnumerator6`
              (set `self.Unlocked` (+ _unlocked_2 1))))
          (`/Engine/EditorBlueprintResources/StandardMacros.CompareInt` _unlocked 7
            (:`>`
              (`KismetSystemLibrary.PrintString` (`KismetStringLibrary.Conv_IntToString` _unlocked)))
            (:`==`
              (`KismetSystemLibrary.PrintString` "would you look at that, you opened the fence")
              (set `self.Unlocked` 0)
              (`self.K2_DestroyActor`))
            (:`<`
              (`KismetSystemLibrary.PrintString` (`KismetStringLibrary.Conv_IntToString` _unlocked))))))
      (:`CastFailed`
        (`KismetSystemLibrary.PrintString` "FAIL")))))

(fn `UserConstructionScript`)