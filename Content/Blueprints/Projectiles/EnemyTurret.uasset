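; EnemyTurret is a turret actor that automatically fires projectiles at a fixed interval.
; Tick accumulates elapsed time and, on reaching RateOfFire, subtracts that interval to keep the leftover time and spawns an EnemyProjectileClass actor at the Arrow component's world transform.
; Each spawn always succeeds regardless of collision and receives the turret's projectile speed and gravity scale, with no targeting or aiming logic.
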(event `self.ReceiveTick`
  (params (DeltaSeconds :type "Float (single-precision)"))
  (bind _output_get (set `self.ElapsedTime` (+ DeltaSeconds (`self.ElapsedTime`))))
  (if (>= _output_get (`self.RateOfFire`))
    (set `self.ElapsedTime` (- (`self.ElapsedTime`) (`self.RateOfFire`)))
    (`|SpawnActorFromClass` (`self.EnemyProjectileClass`) (`SceneComponent.K2_GetComponentToWorld` (`self.Arrow`)) "AlwaysSpawn" "OverrideRootScale" null (`self.ProjectileSpeed`) (`self.ProjectileGravityScale`))))

(fn `UserConstructionScript`)